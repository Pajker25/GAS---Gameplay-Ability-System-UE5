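; Reactive Gameplay Ability that manages delayed stamina regeneration on the avatar actor.
; Once activated, it keeps listening for attribute changes and compares each new value with the last stored one.
; A drop removes the active regen effect by handle, then reapplies GE_StatusStaminaRegen after a short delay.
; Otherwise, the effect is removed once the value reaches a compared attribute, presumably max stamina.
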(event Ability|EventActivateAbility
  (Variables|Default|SetOldStamina (.ReturnValue (Ability|Attribute|GetFloatAttribute (Ability|GetAvatarActorfromActorInfo) "(AttributeName=\"Stamina\",Attribute=/Script/NexusGAS.BasicAttributeSet:Stamina,AttributeOwner=\"/Script/CoreUObject.Class'/Script/NexusGAS.BasicAttributeSet'\")")))
  (|WaitforAttributeChange :Attribute "(AttributeName=\"Stamina\",Attribute=/Script/NexusGAS.BasicAttributeSet:Stamina,AttributeOwner=\"/Script/CoreUObject.Class'/Script/NexusGAS.BasicAttributeSet'\")" :TriggerOnce false :OptionalExternalOwner 0
    (:OnChange
      (bind _output_get (Variables|Default|SetNewStamina (.ReturnValue (Ability|Attribute|GetFloatAttribute (Ability|GetAvatarActorfromActorInfo) "(AttributeName=\"Stamina\",Attribute=/Script/NexusGAS.BasicAttributeSet:Stamina,AttributeOwner=\"/Script/CoreUObject.Class'/Script/NexusGAS.BasicAttributeSet'\")"))))
      (Utilities|FlowControl|Sequence
        (:then_0
          (if (< _output_get (Variables|Default|GetOldStamina))
            (Ability|RemoveGameplayEffectFromOwnerWithHandle (Variables|Default|GetStaminaRegenEffectHandle))
            (Ability|Tasks|WaitDelay 1.0
              (:OnFinish
                (bind _returnvalue (Ability|ApplyGameplayEffectToOwner "/Game/GameplayAbilitySystem/Effects/GE_StatusStaminaRegen.GE_StatusStaminaRegen_C"))
                (Variables|Default|SetStaminaRegenEffectHandle _returnvalue)
                (Variables|Default|SetOldStamina (Variables|Default|GetNewStamina))))
            (elif (>= (Variables|Default|GetNewStamina) (.ReturnValue (Ability|Attribute|GetFloatAttribute (Ability|GetAvatarActorfromActorInfo) "(AttributeName=\"MaxStamina\",Attribute=/Script/NexusGAS.BasicAttributeSet:MaxStamina,AttributeOwner=\"/Script/CoreUObject.Class'/Script/NexusGAS.BasicAttributeSet'\")")))
              (Ability|RemoveGameplayEffectFromOwnerWithHandle (Variables|Default|GetStaminaRegenEffectHandle)))))
        (:then_1
          (Variables|Default|SetOldStamina (Variables|Default|GetNewStamina)))))))