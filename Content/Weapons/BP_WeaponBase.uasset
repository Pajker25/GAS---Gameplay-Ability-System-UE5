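; BP_WeaponBase is a base weapon Blueprint that delivers Gameplay Ability System effects through timed hit detection.
; HitScanStart stores an effect spec, clears the hit list and starts a looping timer at about 60 Hz, which HitScanEnd stops.
; HitScan sphere-traces between two trace points for pawns, excluding the instigator, and applies the effect once per target with an ability system.
; A helper also exposes the spawn point location.
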(event Custom|HitScanEnd
  (Utilities|Time|ClearandInvalidateTimerbyHandle (Variables|Default|GetHitScanTimer)))

(event Custom|HitScan
  (bind _outhits (Collision|MultiSphereTraceForObjects (Transformation|GetWorldLocation (Variables|Default|GetTraceStart)) (Transformation|GetWorldLocation (Variables|Default|GetTraceEnd)) (Variables|Default|GetHitScanRadius) (Utilities|Array|MakeArray "ObjectTypeQuery3") false (Utilities|Array|MakeArray (Variables|Actor|GetInstigator)) "ForDuration" true "(R=1.000000,G=0.000000,B=0.000000,A=1.000000)" "(R=0.000000,G=1.000000,B=0.000000,A=1.000000)" 0.1))
  (for _array_element _outhits
    (Utilities|IsValid (Ability|GetAbilitySystemComponent (.HitActor (Collision|BreakHitResult _array_element)))
      (:Is%20Valid
        (if (not (Utilities|Array|ContainsItem (Variables|Default|GetHitActors) (.HitActor (Collision|BreakHitResult _array_element))))
          (Utilities|Array|AddUnique (Variables|Default|GetHitActors) (.HitActor (Collision|BreakHitResult _array_element)))
          (GameplayEffects|ApplyGameplayEffectSpecToTarget (Ability|GetAbilitySystemComponent (Game|GetInstigator)) (Variables|Default|GetEffectSpecHandle) (Ability|GetAbilitySystemComponent (.HitActor (Collision|BreakHitResult _array_element)))))))))

(event Custom|HitScanStart
  (params (EffectSpecHandle :type Gameplay%20Effect%20Spec%20Handle%20Structure))
  (Variables|Default|SetEffectSpecHandle EffectSpecHandle)
  (Utilities|Array|Clear (Variables|Default|GetHitActors))
  (bind _returnvalue (Utilities|Time|SetTimerbyEvent (EventDispatchers|CreateEvent :!event Custom|HitScan) 0.016667 true))
  (Variables|Default|SetHitScanTimer _returnvalue))

(fn ConstructionScript)

(fn GetSpawnPointLocation
  (return (Transformation|GetWorldLocation (Variables|Default|GetSpawnPoint))))